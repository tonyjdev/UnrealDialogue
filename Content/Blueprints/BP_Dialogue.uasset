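; BP_Dialogue is a Blueprint that displays the UI_DialogueSystem dialogue widget to the player.
; On BeginPlay it creates the widget, stores a reference, adds it to the viewport as visible, and switches input to UI-only with the mouse cursor shown.
; Pressing H makes the stored widget visible again and returns input focus to it.
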(event EventBeginPlay
  (bind _returnvalue (UserInterface|CreateWidget "/Game/UI/UI_DialogueSystem.UI_DialogueSystem_C"))
  (Variables|Default|SetUI_Dialogue_Ref _returnvalue)
  (UserInterface|Viewport|AddtoViewport _returnvalue 0)
  (Widget|SetVisibility _returnvalue "Visible")
  (Input|SetInputModeUIOnly (Game|GetPlayerController 0) _returnvalue "DoNotLock")
  (Variables|/Script/Engine.PlayerController|SetbShowMouseCursor (Game|GetPlayerController 0) true))

(event Input|KeyboardEvents|H
  (params (Key :type Key%20Structure :default "None"))
  (bind _ui_dialogue_ref (Variables|Default|GetUI_Dialogue_Ref))
  (:Pressed
    (Widget|SetVisibility _ui_dialogue_ref "Visible")
    (Input|SetInputModeUIOnly (Game|GetPlayerController 0) _ui_dialogue_ref "DoNotLock")))

(fn ConstructionScript)